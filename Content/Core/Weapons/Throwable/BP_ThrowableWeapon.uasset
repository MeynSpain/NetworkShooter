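; BP_ThrowableWeapon is a throwable weapon that launches a projectile when used.
; UseWeapon defers to the parent check and, on success, calls SpawnThrowProjectile and reports the result.
; The projectile of the configured class spawns ahead of the instigating BP_PlayerCharacter's camera, along the owner's forward vector with a small rotation offset.
; It receives the weapon's damage, the weapon as owner and the same instigator.
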(fn `SpawnThrowProjectile`
  (bind _asbp_player_character (cast `/Game/Core/Player/Character/BP_PlayerCharacter` (`self.GetInstigator`)))
  (`|SpawnActorFromClass` (`self.ProjectileClass`) (`KismetMathLibrary.MakeTransform` (+ (`SceneComponent.K2_GetComponentLocation` (`/Game/Core/Player/Character/BP_PlayerCharacter.Camera` _asbp_player_character)) (* (`self.GetActorForwardVector` (`self.GetOwner`)) 70.0)) (`KismetMathLibrary.ComposeRotators` (`KismetMathLibrary.Conv_VectorToRotator` (`self.GetActorForwardVector` (`self.GetOwner`))) (struct :`Pitch` 10.0))) "Undefined" "OverrideRootScale" self (`self.Damage`) (`self.GetInstigator`)))

(fn `UserConstructionScript`
  (`parent.UserConstructionScript`))

(fn `UseWeapon`
  (returns (bUsed :type Boolean))
  (bind _bused (`parent.UseWeapon`))
  (if _bused
    (`self.SpawnThrowProjectile`)
    (return true)
    (else
      (return false))))