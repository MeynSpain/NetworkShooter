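; Ranged firearm weapon extending a parent weapon class, firing either a projectile or a hitscan trace with point damage, depending on whether ProjectileClass is set.
; Both modes start at the player camera and follow the owner's forward vector; traces draw debug shapes.
; An empty magazine sets Reloading, whose OnRep runs a timed reload on authority, refilling toward the class-default ammo from TotalAmmo.
; Reloading blocks weapon use.
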(event `Debug_DrawServerTrace`
  (params (Start :type "Vector Structure") (End :type "Vector Structure") (Hit :type "Vector Structure"))
  (`KismetSystemLibrary.DrawDebugLine` Start End (struct :`R` 0.402 :`G` 0.329676 :`A` 1.0) 5.0 2.0)
  (`KismetSystemLibrary.DrawDebugSphere` Hit 15.0 8 (struct :`R` 1.0 :`B` 0.019891 :`A` 1.0) 5.0 2.0))

(fn `Fire Trace`
  (returns (Hit :type "HitResult Structure"))
  (bind _asbp_player_character (cast `/Game/Core/Player/Character/BP_PlayerCharacter` (`self.GetInstigator`))
    (:`then`
      (bind _returnvalue (`SceneComponent.K2_GetComponentLocation` (`/Game/Core/Player/Character/BP_PlayerCharacter.Camera` _asbp_player_character)))
      (bind _outhit (`KismetSystemLibrary.LineTraceSingleForObjects` _returnvalue (+ _returnvalue (* (`self.GetActorForwardVector` (`self.GetOwner`)) 10000.0)) (`|MakeArray` "ObjectTypeQuery1" "ObjectTypeQuery2" "ObjectTypeQuery3" :!type "EObjectTypeQuery Enum") false (`|MakeArray` self (`self.GetInstigator`) :!type "Actor Object Reference") "ForDuration"))
      (bind (_bblockinghit _binitialoverlap _time _distance _location _impactpoint _normal _impactnormal _physmat _hitactor _hitcomponent _hitbonename _hititem _elementindex _faceindex _tracestart _traceend) (`GameplayStatics.BreakHitResult` _outhit))
      (`self.Debug_DrawServerTrace` _tracestart _traceend _location))
    (:`CastFailed`
      _))
  (return _outhit))

(fn `IsAbleToReaload`
  (returns (ReturnValue :type Boolean))
  (return (and (!= (`.CurrentAmmo` (defaults `Object` (`GameplayStatics.GetObjectClass` self))) (`self.CurrentAmmo`)) (> (`self.TotalAmmo`) 0) (not (`KismetSystemLibrary.K2_IsValidTimerHandle` (`self.ReloadTimer`))))))

(fn `IsAbleToUseWeapon`
  (returns (bCanUse :type Boolean))
  (return (and (`parent.IsAbleToUseWeapon`) (not (`self.bReloading`)))))

(fn `OnRep_bReloading`
  (`/Engine/EditorBlueprintResources/ActorMacros.Switch Has Authority`
    (:`Authority`
      (if (`self.bReloading`)
        (if (`self.IsAbleToReaload`)
          (`/Game/Core/Libs/Functions/BPL_Functions_Debug.Print Message` "Reloading..." (struct :`R` 0.019187 :`G` 0.035779 :`B` 0.245 :`A` 1.0) 2.0)
          (bind _returnvalue (`KismetSystemLibrary.K2_SetTimer` null "ReloadFinished" (`self.ReloadTime`)))
          (set `self.ReloadTimer` _returnvalue)
          (set `self.AmmoToReload` (`KismetMathLibrary.Min` (- (`.CurrentAmmo` (defaults `Object` (`GameplayStatics.GetObjectClass` self))) (`self.CurrentAmmo`)) (`self.TotalAmmo`)))
          (else
            (set `self.bReloading` false)
            (`/Game/Core/Libs/Functions/BPL_Functions_Debug.Print Message` "Not Able to Reload" (struct) 2.0 true)))))))

(fn `ReloadFinished`
  (set `self.bReloading` false)
  (set `self.CurrentAmmo` (+ (`self.CurrentAmmo`) (`self.AmmoToReload`)))
  (set `self.TotalAmmo` (- (`self.TotalAmmo`) (`self.AmmoToReload`)))
  (`KismetSystemLibrary.K2_ClearAndInvalidateTimerHandle` (`self.ReloadTimer`)))

(fn `Spawn Shoot Projectile`
  (bind _asbp_player_character (cast `/Game/Core/Player/Character/BP_PlayerCharacter` (`self.GetInstigator`)))
  (`|SpawnActorFromClass` (`self.ProjectileClass`) (`KismetMathLibrary.MakeTransform` (+ (`SceneComponent.K2_GetComponentLocation` (`/Game/Core/Player/Character/BP_PlayerCharacter.Camera` _asbp_player_character)) (* (`self.GetActorForwardVector` (`self.GetOwner`)) 70.0)) (`KismetMathLibrary.Conv_VectorToRotator` (`self.GetActorForwardVector` (`self.GetOwner`)))) "Undefined" "OverrideRootScale" self (`self.Damage`) (`self.GetInstigator`)))

(fn `UserConstructionScript`
  (`parent.UserConstructionScript`))

(fn `UseWeapon`
  (returns (bUsed :type Boolean))
  (bind _bused (`parent.UseWeapon`))
  (`/Game/Core/Libs/Functions/BPL_Functions_Debug.Print Message` (`KismetStringLibrary.Concat_StrStr` (`KismetStringLibrary.Conv_IntToString` (`self.CurrentAmmo`)) " / " (`KismetStringLibrary.Conv_IntToString` (`self.TotalAmmo`))) (struct :`G` 0.046825 :`B` 0.35 :`A` 1.0) 1.0)
  (if _bused
    (if (`KismetSystemLibrary.IsValidClass` (`self.ProjectileClass`))
      (`self.Spawn Shoot Projectile`)
      (return true)
      (else
        (bind _hit (`self.Fire Trace`))
        (bind (_bblockinghit _binitialoverlap _time _distance _location _impactpoint _normal _impactnormal _physmat _hitactor _hitcomponent _hitbonename _hititem _elementindex _faceindex _tracestart _traceend) (`GameplayStatics.BreakHitResult` _hit))
        (`GameplayStatics.ApplyPointDamage` _hitactor (`self.Damage`) (`KismetMathLibrary.GetDirectionUnitVector` _traceend _tracestart) _hit (`self.GetInstigatorController`) self)
        (return true)))
    (elif (and (<= (`self.CurrentAmmo`) 0) (> (`self.TotalAmmo`) 0))
      (set `self.bReloading` true)
      (return false)
      (else
        (return false)))))