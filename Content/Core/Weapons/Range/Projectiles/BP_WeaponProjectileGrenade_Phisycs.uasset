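; Physics-driven grenade weapon projectile that explodes after a timed fuse.
; On BeginPlay the server applies a forward throw impulse to the box collision and starts a timer for Explode.
; Explode deals full radial damage, blocked by WorldStatic, then destroys the actor.
; Remote copies play the explosion particle and sound when Destroyed fires, so destruction itself carries the effect to clients.
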(event `self.ReceiveBeginPlay`
  ;[1 1 1] Begin Play. Add Impulse to grenade
  (`/Engine/EditorBlueprintResources/ActorMacros.Switch Has Authority`
    (:`Authority`
      (`PrimitiveComponent.AddImpulse` (`self.BoxCollision`) (* (`self.GetActorForwardVector`) (`self.ThrowPower`)) "None" false)
      (`KismetSystemLibrary.K2_SetTimer` null "Explode" (`self.ExplosionDelay`)))))

(event `self.ReceiveDestroyed`
  (bind _returnvalue (`self.K2_GetActorLocation`))
  (`parent.ReceiveDestroyed`)
  (`/Engine/EditorBlueprintResources/ActorMacros.Switch Has Authority`
    (:`Remote`
      (`GameplayStatics.SpawnEmitterAtLocation` "/Game/MilitaryWeapDark/FX/P_Grenade_Explosion_01.P_Grenade_Explosion_01" _returnvalue)
      (`GameplayStatics.PlaySoundAtLocation` "/Game/MilitaryWeapDark/Sound/GrenadeLauncher/GrenadeLauncher_Explosion_Cue.GrenadeLauncher_Explosion_Cue" _returnvalue (struct) 1.0 1.0 0.0 null null null))))

(fn `Explode`
  (`GameplayStatics.ApplyRadialDamage` :`BaseDamage` (`self.Damage`) :`Origin` (`self.K2_GetActorLocation`) :`DamageRadius` (`self.ExplosionRadius`) :`DamageCauser` self :`InstigatedByController` (`self.GetInstigatorController`) :`bDoFullDamage` true :`DamagePreventionChannel` "ECC_WorldStatic")
  (`self.K2_DestroyActor`))

(fn `UserConstructionScript`
  (`parent.UserConstructionScript`))