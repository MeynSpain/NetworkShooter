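; Base weapon Blueprint for a replicated, pickup-able weapon; interacting hands it to the character's BPCWeaponManager.
; UseWeapon checks ammo and cooldown, spends a round and starts a rate timer, whose expiry re-fires while auto fire is held.
; OnRep_WeaponOwner handles pickup and drop by updating instigator, owner, collision and attachment.
; On pickup, authority attaches to the character, while remotes socket the current weapon to the visible mesh and hide others.
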(fn `Interact`
  (params (PlayerCharacter :type "/Game/Core/Player/Character/BP_PlayerCharacter Object Reference"))
  (returns (Success :type Boolean))
  (`/Game/Core/Componets/Player/BPC_WeaponManager.AddWeapon` (`/Game/Core/Player/Character/BP_PlayerCharacter.BPC_WeaponManager` PlayerCharacter) self)
  (return false))

(fn `IsAbleToUseWeapon`
  (returns (bCanUse :type Boolean))
  (return (and (> (`self.CurrentAmmo`) 0) (not (`self.bUseFreezedByRate`)))))

(fn `OnRep_WeaponOwner`
  (bind _weaponowner (`self.WeaponOwner`)
    (:`then`
      (bind _output_get (set `self.Instigator` _weaponowner))
      (`self.SetOwner` (`Pawn.GetController` _output_get))
      ;[1 1 1] При подбирании
      (`self.SetActorEnableCollision` false)
      (`/Engine/EditorBlueprintResources/ActorMacros.Switch Has Authority`
        (:`Authority`
          (`self.K2_AttachToActor` (`self.WeaponOwner`) "None" "SnapToTarget" "SnapToTarget" "KeepRelative"))
        (:`Remote`
          (if (!= (`/Game/Core/Componets/Player/BPC_WeaponManager.CurrentWeapon` (`/Game/Core/Player/Character/BP_PlayerCharacter.BPC_WeaponManager` (`self.WeaponOwner`))) self)
            (`self.SetActorHiddenInGame` true)
            (else
              ;[1 1 1] Потому что почему то оружие переатачивается
              (`self.K2_AttachToComponent` (`/Game/Core/Player/Character/BP_PlayerCharacter.GetVisibleMesh` (`self.WeaponOwner`)) "SKT_Weapon" "SnapToTarget" "SnapToTarget" "KeepRelative"))))))
    (:`else`
      ;[1 1 1] При выбрасывании оружия
      (`self.K2_DetachFromActor` "KeepRelative")
      (`self.SetActorHiddenInGame` false)
      (`self.SetActorEnableCollision` true)
      (set `self.Instigator` null)
      (`self.SetOwner` null))))

(fn `SetWeaponOwner`
  (params (PlayerCharacter :type Boolean)))

(fn `StopRateDelay`
  (set `self.bUseFreezedByRate` false)
  (if (and (`self.bAutoFire`) (`self.bFireActive`))
    (`self.UseWeapon`)))

(fn `StopUseWeapon`
  (set `self.bFireActive` false))

(fn `UserConstructionScript`)

(fn `UseWeapon`
  (returns (bUsed :type Boolean))
  (if (`self.IsAbleToUseWeapon`)
    (`/Engine/EditorBlueprintResources/StandardMacros.DecrementInt` (`self.CurrentAmmo`)
      (:`  `
        ;[1 1 1] Логика не зависнет на этом таймере, тут просто активируется таймер, но сама логика пойдет дальше. После того как таймер истечет, выполнится определенное действие.
        (`KismetSystemLibrary.K2_SetTimer` null "StopRateDelay" (/ 1.0 (`self.UseRate`)))
        (set `self.bUseFreezedByRate` true)
        (if (`self.bAutoFire`)
          (set `self.bFireActive` true))
        (return true)))
    (else
      (set `self.bFireActive` false)
      (return false))))