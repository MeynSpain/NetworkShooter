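; BP_MeleeWeapon is a melee weapon that deals point damage to what it strikes in front of its wielder.
; When the parent UseWeapon succeeds, it sphere-traces from the player camera along the owner's forward vector out to Radius, then applies Damage to the hit actor.
; The trace requires a BP_PlayerCharacter instigator and draws debug shapes.
; Availability depends only on the UseFreezedByRate rate-limit flag.
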(fn `GerOverlapInfo`
  (returns (Hit :type "HitResult Structure"))
  (bind _asbp_player_character (cast `/Game/Core/Player/Character/BP_PlayerCharacter` (`self.GetInstigator`))
    (:`then`
      (bind _returnvalue (`SceneComponent.K2_GetComponentLocation` (`/Game/Core/Player/Character/BP_PlayerCharacter.Camera` _asbp_player_character)))
      (bind _outhit (`KismetSystemLibrary.SphereTraceSingleForObjects` _returnvalue (+ _returnvalue (* (`self.GetActorForwardVector` (`self.GetOwner`)) (`self.Radius`))) 30.0 (`|MakeArray` "ObjectTypeQuery1" "ObjectTypeQuery2" "ObjectTypeQuery3" :!type "EObjectTypeQuery Enum") false (`|MakeArray` self (`self.GetInstigator`) :!type "Actor Object Reference") "ForDuration"))
      (return _outhit))
    (:`CastFailed`
      (return))))

(fn `IsAbleToUseWeapon`
  (returns (bCanUse :type Boolean))
  (return (not (`self.bUseFreezedByRate`))))

(fn `UserConstructionScript`
  (`parent.UserConstructionScript`))

(fn `UseWeapon`
  (returns (bUsed :type Boolean))
  (bind _bused (`parent.UseWeapon`))
  (if _bused
    (bind _hit (`self.GerOverlapInfo`))
    (bind (_bblockinghit _binitialoverlap _time _distance _location _impactpoint _normal _impactnormal _physmat _hitactor _hitcomponent _hitbonename _hititem _elementindex _faceindex _tracestart _traceend) (`GameplayStatics.BreakHitResult` _hit))
    (`GameplayStatics.ApplyPointDamage` _hitactor (`self.Damage`) (`KismetMathLibrary.GetDirectionUnitVector` _traceend _tracestart) _hit (`self.GetInstigatorController`) self)
    (return true)
    (else
      (return false))))