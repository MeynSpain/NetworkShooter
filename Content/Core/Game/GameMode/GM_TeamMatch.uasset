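; Team match game mode that adds team-based spawning, damage rules and scoring to its parent mode.
; Spawn selection keeps free BP_GamePlayerStart actors matching the player's team, and damage between teammates requires AllowFriendlyFire.
; Deaths add a point to the instigator's team in BP_GameState_Team, or subtract one for same-team kills.
; With LimitByTeamPoints on, a death stops the round once the instigator's team reaches TeamPointsLimit.
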(fn `CharacterDead`
  (params (DeadCharacter :type "/Game/Core/Player/Character/BP_PlayerCharacter Object Reference") (DeathInstigater :type "/Game/Core/Player/Controller/BP_PlayerController Object Reference") (DeathCausedBy :type "Actor Object Reference"))
  (`parent.CharacterDead` DeadCharacter DeathInstigater DeathCausedBy)
  (if (`self.bLimitByTeamPoints`)
    (if (>= (`/Game/Core/Game/State/BP_GameState_Team.GetTeamPoints` (cast `/Game/Core/Game/State/BP_GameState_Team` (`GameplayStatics.GetGameState`) :!pure true) (`/Game/Core/Player/State/BP_PlayerState_Team.Team` (`/Game/Core/Libs/Functions/BPL_Functions_GlobalGetters.GetTeamPlayerStateByController` DeathInstigater))) (`self.TeamPointsLimit`))
      (`self.StopRound` "Team points limit"))))

(fn `GetFreeSpawnPoints`
  (params (Player :type "/Game/Core/Player/Controller/BP_PlayerController Object Reference"))
  (returns (FreeSpawns :type "Array of /Game/Core/Game/Start/BP_GamePlayerStart Object Reference"))
  (locals (L_FreePoints :type "Array of /Game/Core/Game/Start/BP_GamePlayerStart Object Reference"))
  (bind _outactors (`GameplayStatics.GetAllActorsOfClass` "/Game/Core/Game/Start/BP_GamePlayerStart.BP_GamePlayerStart_C"))
  (for _array_element _outactors
    (if (and (`/Game/Core/Game/Start/BP_GamePlayerStart.IsFree` _array_element) (`|EnumEquality` (`/Game/Core/Game/Start/BP_GamePlayerStart.Team` _array_element) (`/Game/Core/Player/State/BP_PlayerState_Team.Team` (`/Game/Core/Libs/Functions/BPL_Functions_GlobalGetters.GetTeamPlayerStateByController` Player))))
      (`KismetArrayLibrary.Array_Add` (`local.L_FreePoints`) _array_element)))
  (return (`local.L_FreePoints`)))

(fn `ShouldDamagePlayer`
  (params (Character :type "/Game/Core/Player/Controller/BP_PlayerController Object Reference") (Instigator :type "/Game/Core/Player/Controller/BP_PlayerController Object Reference"))
  (returns (bOut :type Boolean))
  (if (`self.bAllowFriendlyFire`)
    (return true)
    (else
      (return (`|EnumInequality` (`/Game/Core/Player/State/BP_PlayerState_Team.Team` (`/Game/Core/Libs/Functions/BPL_Functions_GlobalGetters.GetTeamPlayerStateByController` Character)) (`/Game/Core/Player/State/BP_PlayerState_Team.Team` (`/Game/Core/Libs/Functions/BPL_Functions_GlobalGetters.GetTeamPlayerStateByController` Instigator)))))))

(fn `UpdateDeathPoints`
  (params (Player :type "/Game/Core/Player/Controller/BP_PlayerController Object Reference") (InstigatorPlayer :type "/Game/Core/Player/Controller/BP_PlayerController Object Reference"))
  (locals (L_DeadPlayer :type "/Game/Core/Player/Controller/BP_PlayerController Object Reference") (L_PlayerDeathInstigator :type "/Game/Core/Player/Controller/BP_PlayerController Object Reference"))
  (bind _asbp_game_state_team (cast `/Game/Core/Game/State/BP_GameState_Team` (`GameplayStatics.GetGameState`) :!pure true))
  (set `local.L_DeadPlayer` Player)
  (bind _output_get (set `local.L_PlayerDeathInstigator` InstigatorPlayer))
  (`parent.UpdateDeathPoints` (`local.L_DeadPlayer`) (`local.L_PlayerDeathInstigator`))
  (if (`/Game/Core/Libs/Functions/BPL_Functions_GlobalGetters.IsAnotherTeam` (`local.L_DeadPlayer`) (`local.L_PlayerDeathInstigator`))
    (bind _team (`/Game/Core/Player/State/BP_PlayerState_Team.Team` (`/Game/Core/Libs/Functions/BPL_Functions_GlobalGetters.GetTeamPlayerStateByController` _output_get)))
    (`/Game/Core/Game/State/BP_GameState_Team.Add Team Points` _asbp_game_state_team _team 1)
    (else
      (`/Game/Core/Game/State/BP_GameState_Team.Add Team Points` _asbp_game_state_team _team -1))))

(fn `UserConstructionScript`
  (`parent.UserConstructionScript`))