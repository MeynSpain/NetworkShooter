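; Deathmatch game mode that can end the round when a player reaches a kill limit.
; It extends its parent's CharacterDead, then, if the kill limit is enabled and the instigator is valid, reads that player's Kills from BP_PlayerState.
; Reaching the configured kills to win calls StopRound with a KillLimit reason and prints a game-over message.
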(fn `CharacterDead`
  (params (DeadCharacter :type "/Game/Core/Player/Character/BP_PlayerCharacter Object Reference") (DeathInstigater :type "/Game/Core/Player/Controller/BP_PlayerController Object Reference") (DeathCausedBy :type "Actor Object Reference"))
  (`parent.CharacterDead` DeadCharacter DeathInstigater DeathCausedBy)
  (`/Engine/EditorBlueprintResources/StandardMacros.IsValid` DeathInstigater
    (:`Is Valid`
      (if (`self.bLimitByKills`)
        (if (>= (`/Game/Core/Player/State/BP_PlayerState.Kills` (cast `/Game/Core/Player/State/BP_PlayerState` (`Controller.PlayerState` DeathInstigater) :!pure true)) (`self.KiilsToWin`))
          (`self.StopRound` "KillLimit")
          (`KismetSystemLibrary.PrintString` "GAME OVER"))))))

(fn `UserConstructionScript`
  (`parent.UserConstructionScript`))