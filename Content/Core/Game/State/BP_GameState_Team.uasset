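; Team game state that tracks score for Team A and Team B.
; BeginPlay sizes PointsArray to the TeamPoints map, and AddTeamPoints adds a value to both the map and the team's array slot.
; GetTeamPoints reads only the array, mapping each team enum to a fixed index.
; A debug print of both scores sits unconnected in the event graph.
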(event `self.ReceiveBeginPlay`
  (`parent.ReceiveBeginPlay`)
  (`KismetArrayLibrary.Array_Resize` (`self.PointsArray`) (`BlueprintMapLibrary.Map_Length` (`self.TeamPoints`))))

(event `self.ReceiveTick`
  (params (DeltaSeconds :type "Float (single-precision)")))

(fn `Add Team Points`
  (params (Team :type "/Game/Data/Enums/ETeam Enum" :default "NewEnumerator0") (Value :type Integer))
  (locals (L_Value :type Integer))
  (bind _returnvalue (select `/Game/Data/Enums/ETeam` Team :`NewEnumerator1` 1))
  (bind _teampoints (`self.TeamPoints`))
  (set `local.L_Value` Value)
  (`BlueprintMapLibrary.Map_Add` _teampoints Team (+ (`BlueprintMapLibrary.Map_Find` _teampoints Team) (`local.L_Value`)))
  (`KismetArrayLibrary.Array_Set` (`self.PointsArray`) _returnvalue (+ (`|GetArrayItem` (`self.PointsArray`) _returnvalue) (`local.L_Value`)) true))

(fn `GetTeamPoints`
  (params (Team :type "/Game/Data/Enums/ETeam Enum" :default "NewEnumerator0"))
  (returns (Points :type Integer))
  (return (`|GetArrayItem` (`self.PointsArray`) (select `/Game/Data/Enums/ETeam` Team :`NewEnumerator1` 1))))

(fn `UserConstructionScript`
  (`parent.UserConstructionScript`))