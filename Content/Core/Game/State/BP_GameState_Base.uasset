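; Base GameState that relays round start and end from GM_BaseGameMode and tracks round time.
; On the server it binds to the game mode's round events and sets RoundInProgress.
; Its RepNotify broadcasts RoundStarted and starts or clears a server-side one-second timer, which calls TimeEnded once RoundTime reaches the mode's TimeLimit.
; RoundEnded goes out by multicast with a reason, and debug prints remain, including one every Tick.
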(event `self.ReceiveBeginPlay`
  ;[1 1 1] Раньше здесь стоя switch has authority
  (if (`KismetSystemLibrary.IsServer`)
    (`KismetSystemLibrary.PrintString` "ПОчему то прошел")
    (bind _asgm_base_game_mode (cast `/Game/Core/Game/GameMode/GM_BaseGameMode` (`GameplayStatics.GetGameMode`)))
    (add `/Game/Core/Game/GameMode/GM_BaseGameMode.RoundEnded` _asgm_base_game_mode (delegate `OnRoundEnded`))
    (bind _asgm_base_game_mode_2 (cast `/Game/Core/Game/GameMode/GM_BaseGameMode` (`GameplayStatics.GetGameMode`)))
    (add `/Game/Core/Game/GameMode/GM_BaseGameMode.RoundStarted` _asgm_base_game_mode_2 (delegate `OnRoundStarted`))))

(event `OnRoundEnded`
  (params (Reason :type String))
  (`self.Multicast-RoundEnd` Reason)
  (set `self.bRoundInProgress` false))

(event `Multicast-RoundEnd`
  (params (Reason :type String))
  (`self.RoundEnded` Reason))

(event `OnRoundStarted`
  (set `self.bRoundInProgress` true))

(event `Multicast-RoundStart`
  (`self.RoundStarted`))

(event `self.ReceiveTick`
  (params (DeltaSeconds :type "Float (single-precision)"))
  (`KismetSystemLibrary.PrintString` (`KismetStringLibrary.Concat_StrStr` "GameState: " (`KismetSystemLibrary.GetDisplayName` self)) true true (struct :`R` 1.0 :`B` 0.643089 :`A` 1.0) 0.0))

(fn `OnRep_bRoundInProgress`
  (if (`self.bRoundInProgress`)
    (`self.RoundStarted`)
    (`/Engine/EditorBlueprintResources/ActorMacros.Switch Has Authority`
      (:`Authority`
        (`KismetSystemLibrary.PrintString` "Раунд начался")
        (`self.StartRoundTimer`)))
    (else
      (`/Engine/EditorBlueprintResources/ActorMacros.Switch Has Authority`
        (:`Authority`
          (`KismetSystemLibrary.PrintString` "Раунд закончился")
          (`KismetSystemLibrary.K2_ClearAndInvalidateTimerHandle` (`self.TickTimer`)))))))

(fn `RoundTimeTick`
  (set `self.RoundTime` (+ (`self.RoundTime`) (`KismetMathLibrary.MakeTimespan` 0 0 0 1)))
  (if (>= (`self.RoundTime`) (`/Game/Core/Game/GameMode/GM_BaseGameMode.TimeLimit` (cast `/Game/Core/Game/GameMode/GM_BaseGameMode` (`GameplayStatics.GetGameMode`) :!pure true)))
    (`self.TimeEnded`)))

(fn `StartRoundTimer`
  (bind _returnvalue (`KismetSystemLibrary.K2_SetTimer` null "RoundTimeTick" 1.0 true))
  (set `self.TickTimer` _returnvalue))

(fn `UserConstructionScript`)