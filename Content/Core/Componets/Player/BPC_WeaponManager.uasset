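; Player weapon manager component that spawns, stores and switches the character's weapons.
; CreateWeapon spawns a weapon, files it into main, secondary, special, grenade or melee slots, and attaches it to the character.
; Client-request events set CurrentWeapon by type or by cycling main, secondary and melee.
; CurrentWeapon's OnRep reattaches the previous weapon to the character and the new one to the mesh socket on clients; AddWeapon is an empty stub.
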(event `self.ReceiveBeginPlay`
  ;[1 1 1] Begin Play
  (bind _asbp_player_character (cast `/Game/Core/Player/Character/BP_PlayerCharacter` (`self.GetOwner`))
    (:`then`
      (set `self.Character` _asbp_player_character))
    (:`CastFailed`
      (`KismetSystemLibrary.PrintString` "Failed cast to Player Character in BPC_WeaponManager" true true (struct :`R` 1.0 :`A` 1.0) 3.0))))

(event `SelectWeaponFromClient`
  (params (Type :type "/Game/Data/Enums/EWeaponTypes Enum" :default "NewEnumerator0"))
  ;[1 1 1] Switch Weapons
  (`self.SelectWeapon` Type))

(event `ScrollWeaponFromClient`
  (params (bNext :type Boolean))
  ;[1 1 1] Switch Weapons
  (`self.ScrollWeapon` bNext))

(fn `AddWeapon`)

(fn `Create Weapon`
  (params (Class :type "/Game/Core/Weapons/BP_Weapon_Base Class Reference"))
  (returns (Weapon :type "/Game/Core/Weapons/BP_Weapon_Base Object Reference"))
  (locals (L_SpawnedWeapon :type "/Game/Core/Weapons/BP_Weapon_Base Object Reference"))
  (bind _character (`self.Character`))
  (bind _l_spawnedweapon (`local.L_SpawnedWeapon`))
  (bind _l_spawnedweapon_2 (`local.L_SpawnedWeapon`))
  (bind _returnvalue (`|SpawnActorFromClass` Class (`KismetMathLibrary.MakeTransform` (0.0 0.0 0.0)) "AlwaysSpawn" "OverrideRootScale" (`Pawn.GetController` _character) _character))
  (bind _output_get (set `local.L_SpawnedWeapon` _returnvalue))
  (switch `/Game/Data/Enums/EWeaponTypes` (`/Game/Core/Weapons/BP_Weapon_Base.WeaponType` _output_get)
    (:`NewEnumerator0`
      (set `self.MainWeapon` _l_spawnedweapon))
    (:`NewEnumerator1`
      (set `self.SecondWeapon` _l_spawnedweapon))
    (:`NewEnumerator2`
      (`KismetArrayLibrary.Array_Add` (`self.Specials`) (`local.L_SpawnedWeapon`)))
    (:`NewEnumerator3`
      (`KismetArrayLibrary.Array_Add` (`self.Grenades`) _l_spawnedweapon_2))
    (:`NewEnumerator4`
      (set `self.MeleeWeapon` _l_spawnedweapon_2)))
  (`Actor.K2_AttachToActor` (`local.L_SpawnedWeapon`) (`self.Character`) "None" "SnapToTarget" "SnapToTarget" "KeepRelative" true)
  (return (`local.L_SpawnedWeapon`)))

(fn `OnRep_CurrentWeapon`
  (if (not (`KismetSystemLibrary.IsServer`))
    (bind _clientweaponattached (`self.ClientWeaponAttached`)
      (:`then`
        (`Actor.K2_AttachToActor` _clientweaponattached (`self.Character`) "None" "SnapToTarget" "SnapToTarget" "KeepRelative" true))
      (:`else`
        _))
    (`Actor.K2_AttachToComponent` (`self.CurrentWeapon`) (`/Game/Core/Player/Character/BP_PlayerCharacter.GetVisibleMesh` (`self.Character`)) "SKT_Weapon" "KeepRelative" "KeepRelative" "KeepRelative" true)
    (set `self.ClientWeaponAttached` (`self.CurrentWeapon`))
    (`/Game/Core/Libs/BPL_Functions_Debug.Print Message` "Weapon Attached" (struct :`A` 1.0) 5.0)))

(fn `ScrollWeapon`
  (params (bNext :type Boolean))
  (bind _weapontype (`/Game/Core/Weapons/BP_Weapon_Base.WeaponType` (`self.CurrentWeapon`)))
  (if bNext
    (switch `/Game/Data/Enums/EWeaponTypes` _weapontype
      (:`NewEnumerator0`
        (`self.SelectWeapon` "NewEnumerator1"))
      (:`NewEnumerator1`
        (`self.SelectWeapon` "NewEnumerator4"))
      (:`NewEnumerator4`
        (`self.SelectWeapon` "NewEnumerator0")))
    (else
      (switch `/Game/Data/Enums/EWeaponTypes` _weapontype
        (:`NewEnumerator0`
          (`self.SelectWeapon` "NewEnumerator4"))
        (:`NewEnumerator1`
          (`self.SelectWeapon` "NewEnumerator0"))
        (:`NewEnumerator4`
          (`self.SelectWeapon` "NewEnumerator1"))))))

(fn `SelectWeapon`
  (params (Type :type "/Game/Data/Enums/EWeaponTypes Enum" :default "NewEnumerator0") (Index :type Integer))
  (returns (Weapon :type "/Game/Core/Weapons/BP_Weapon_Base Object Reference"))
  (bind _returnvalue (select `/Game/Data/Enums/EWeaponTypes` Type :`NewEnumerator0` (`self.MainWeapon`) :`NewEnumerator1` (`self.SecondWeapon`) :`NewEnumerator2` (`|GetArrayItem` (`self.Specials`) Index) :`NewEnumerator3` (`|GetArrayItem` (`self.Grenades`) Index) :`NewEnumerator4` (`self.MeleeWeapon`)))
  (`/Engine/EditorBlueprintResources/StandardMacros.IsValid` _returnvalue
    (:`Is Valid`
      (bind _output_get (set `self.CurrentWeapon` _returnvalue))
      (return _output_get))
    (:`Is Not Valid`
      (return (`self.CurrentWeapon`)))))