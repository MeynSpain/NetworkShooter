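; Player health component that tracks health and armor and applies incoming damage to the owning BP_PlayerCharacter.
; On the server it binds to the character's any-damage event and consults the game mode's ShouldDamagePlayer check.
; Armor cuts health damage by up to half, proportional to remaining armor, then drops by the raw damage.
; At zero health it flags the character dead and notifies GM_BaseGameMode with instigator and causer.
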(event Custom|OnPlayerTakeAnyDamage
  (params (DamagedActor :type Actor%20Object%20Reference) (Damage :type Float%20%28single-precision%29) (DamageType :type Damage%20Type%20Object%20Reference) (InstigatedBy :type Controller%20Object%20Reference) (DamageCauser :type Actor%20Object%20Reference))
  ;[1 1 1] Получение урона
  (|ShouldDamage InstigatedBy)
  (CallFunction|DecreaseHelth Damage)
  (CallFunction|PrintMessage "HIt" "(R=0.011826,G=0.030590,B=0.167000,A=1.000000)" 2.0 false)
  ;;[1 1 1] Проверка на смерть
  (if (<= (Variables|Stats|GetHealth) 0.0)
    (Variables|/Game/Core/Player/Character/BP_PlayerCharacter.BP_PlayerCharacter_C|SetbDead (Variables|Character|GetCharacter) true)
    (bind _asgm_base_game_mode (Utilities|Casting|CastToGM_BaseGameMode (Game|GetGameMode)))
    (Default|CharacterDead _asgm_base_game_mode (Variables|Character|GetCharacter) (.AsBP%20Player%20Controller (Utilities|Casting|CastToBP_PlayerController InstigatedBy)) DamageCauser)))

(event EventBeginPlay
  (Variables|Stats|SetHealth (Variables|Stats|GetMaxHealth))
  (Variables|Stats|SetArmor (Variables|Stats|GetMaxArmor))
  (bind _asbp_player_character (Utilities|Casting|CastToBP_PlayerCharacter (Components|GetOwner)))
  (bind _output_get (Variables|Character|SetCharacter _asbp_player_character))
  (if (Networking|IsServer)
    (EventDispatchers|BindEventtoOnTakeAnyDamage _output_get (EventDispatchers|CreateEvent :!event Custom|OnPlayerTakeAnyDamage))))

(fn DecreaseHelth
  (params (Damage :type Float%20%28single-precision%29))
  (LocalVariables|SetL_Damage Damage)
  (Variables|Stats|SetHealth (|(Max(({7E309737-4A99-B841-0EE9-9A846EB831FD}-({1C4906A7-40AB-F400-F290-0DBCB2021317}*(1-({4CE76C34-4E3A-B61E-57AB-65A6FC67B930}/({E3953BE7-4E8A-AE22-5689-06822C03C05D}*2))))),0))))
  (Variables|Stats|SetArmor (|(Max(({4CE76C34-4E3A-B61E-57AB-65A6FC67B930}-{1C4906A7-40AB-F400-F290-0DBCB2021317}),0))))
  ;[1 1 1] Дебажная херня
  (CallFunction|PrintMessage (Utilities|String|Append "Health: " (Utilities|String|ToString(Float) (Variables|Stats|GetHealth))) "(R=0.000000,G=1.000000,B=0.000000,A=1.000000)" 2.0 false))

(fn GetHealth
  (return (Variables|Stats|GetHealth) (Variables|Stats|GetMaxHealth)))

(fn GetArmor
  (return (Variables|Stats|GetArmor) (Variables|Stats|GetMaxArmor)))