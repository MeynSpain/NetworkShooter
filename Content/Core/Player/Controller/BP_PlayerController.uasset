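; Player controller that handles respawning, chat and HUD switching for the player.
; Respawns go through GM_BaseGameMode's SpawnPlayer, either on a timer cancelled by round end or through a server event when a spectator presses Enter and fast respawn is allowed.
; Tab shows the tab screen in place of the HUD or spectate view, depending on alive state.
; T and Escape control chat, and messages post through the game state's chat component.
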(event `self.ReceiveBeginPlay`
  ;[1 1 1] Begin Play
  (bind _asbph_hud_base (cast `/Game/Core/Game/HUD/BPH_HUD_Base` (`self.GetHUD`)))
  (set `self.HUD` _asbph_hud_base))

(event `RoundEndedInRespawn`
  (params (Reason :type String))
  (remove `/Game/Core/Game/GameMode/GM_BaseGameMode.RoundEnded` (`/Game/Core/Libs/Functions/BPL_Functions_GlobalGetters.GetGameMode`) (delegate `RoundEndedInRespawn`))
  (`KismetSystemLibrary.K2_ClearAndInvalidateTimerHandle` (`self.RespawnTimer`)))

(event `Key|Enter`
  (params (Key :type "Key Structure"))
  ;[1 1 1] Respawn Player
  (:`Pressed`
    (cast `/Game/Core/Game/Spectators/BP_GameSpectator_Base` (`self.K2_GetPawn`))
    (`self.Server-Respawn`)))

(event `Server-Respawn`
  ;[1 1 1] Respawn Player
  (bind _asgm_base_game_mode (cast `/Game/Core/Game/GameMode/GM_BaseGameMode` (`GameplayStatics.GetGameMode`)))
  (if (`/Game/Core/Game/GameMode/GM_BaseGameMode.bAllowFastRespawn` _asgm_base_game_mode)
    (`self.Respawn`)))

(event `Key|Tab`
  (params (Key :type "Key Structure"))
  (bind _hud (`self.HUD`))
  (bind _hud_2 (`self.HUD`))
  (bind _hud_3 (`self.HUD`))
  (bind _hud_4 (`self.HUD`))
  (bind _balive (`/Game/Core/Player/State/BP_PlayerState.bAlive` (cast `/Game/Core/Player/State/BP_PlayerState` (`self.PlayerState`) :!pure true)))
  ;[1 1 1] Tab Switch
  (:`Pressed`
    (if _balive
      (`/Game/Core/Game/HUD/BPH_HUD_Base.ToogleTab` _hud_3 true)
      (`/Game/Core/Game/HUD/BPH_HUD_Base.Toogle HUD` _hud_2 false)
      (else
        (`/Game/Core/Game/HUD/BPH_HUD_Base.ToogleTab` _hud_4 true)
        (`/Game/Core/Game/HUD/BPH_HUD_Base.ToogleSpectate` _hud false))))
  (:`Released`
    (if _balive
      (`/Game/Core/Game/HUD/BPH_HUD_Base.ToogleTab` _hud_3 false)
      (`/Game/Core/Game/HUD/BPH_HUD_Base.Toogle HUD` _hud_2 true)
      (else
        (`/Game/Core/Game/HUD/BPH_HUD_Base.ToogleTab` _hud_4 false)
        (`/Game/Core/Game/HUD/BPH_HUD_Base.ToogleSpectate` _hud true)))))

(event `SendChatMessageToServer`
  (params (Message :type Text))
  (`/Game/Core/Componets/Game/BPC_ChatComponent.PostMessage` (`/Game/Core/Game/State/BP_GameState_Base.BPC_ChatComponent` (`/Game/Core/Libs/Functions/BPL_Functions_GlobalGetters.Get Game State`)) Message (cast `/Game/Core/Player/State/BP_PlayerState` (`self.PlayerState`) :!pure true)))

(event `Key|T`
  (params (Key :type "Key Structure"))
  (bind _hud (`self.HUD`))
  (:`Pressed`
    (if (`/Game/Core/Game/HUD/BPH_HUD_Base.IsChatActive` (`self.HUD`))
      (`/Game/Core/Game/HUD/BPH_HUD_Base.ToogleChat` _hud false)
      (else
        (`/Game/Core/Game/HUD/BPH_HUD_Base.ToogleChat` _hud true)))))

(event `Key|Escape`
  (params (Key :type "Key Structure"))
  (:`Pressed`
    (if (`/Game/Core/Game/HUD/BPH_HUD_Base.IsChatActive` (`self.HUD`))
      (`/Game/Core/Game/HUD/BPH_HUD_Base.ToogleChat` (`self.HUD`) false))))

(fn `LaunchRespawnTimer`
  (params (Time :type "Float (double-precision)"))
  (bind _returnvalue (`KismetSystemLibrary.K2_SetTimer` null "Respawn" Time))
  (set `self.RespawnTimer` _returnvalue)
  (add `/Game/Core/Game/GameMode/GM_BaseGameMode.RoundEnded` (`/Game/Core/Libs/Functions/BPL_Functions_GlobalGetters.GetGameMode`) (`|CreateDelegate` :!event `RoundEndedInRespawn`)))

(fn `Respawn`
  (bind _asgm_base_game_mode (cast `/Game/Core/Game/GameMode/GM_BaseGameMode` (`GameplayStatics.GetGameMode`)))
  (`/Game/Core/Game/GameMode/GM_BaseGameMode.SpawnPlayer` _asgm_base_game_mode self))

(fn `SpawnAsSpectator`)

(fn `UserConstructionScript`)